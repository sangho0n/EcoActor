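; BP_OceanCleaning runs the Level 2 ocean-cleaning minigame, a timed challenge to reach a garbage point target.
; BeginPlay caches the game, time-over and mission-complete UIs from widget components, shows the HUD and starts a one-second looping timer.
; CountTime updates the countdown, showing time-over at zero or mission-complete once points reach the target, with UI-only input.
; ShowGarbagePoints stores the score it receives and updates the HUD.
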(event Custom|커스텀%20이벤트_0
  (params (Points :type Integer))
  (Development|PrintText (Utilities|Text|ToText(Integer) Points)))

(event EventBeginPlay
  (Utilities|FlowControl|Sequence
    (:then_0
      (Utilities|FlowControl|Sequence
        (:then_0
          (bind _asbp_oc_game_ui (Utilities|Casting|CastToBP_OC_Game_UI (UserInterface|GetUserWidgetObject (Variables|Default|GetWidget_OC_Game))))
          (Variables|Default|SetBP_OC_Game_UI _asbp_oc_game_ui))
        (:then_1
          (bind _asbp_timeover_ui (Utilities|Casting|CastToBP_Timeover_UI (UserInterface|GetUserWidgetObject (Variables|Default|GetWidget_TimeOver))))
          (Variables|Default|SetBP_TimeOver_UI _asbp_timeover_ui))
        (:then_2
          (bind _asbp_mission_complete_ui (Utilities|Casting|CastToBP_MissionComplete_UI (UserInterface|GetUserWidgetObject (Variables|Default|GetWidget_MissionComplete))))
          (Variables|Default|SetBP_MissionComplete_UI _asbp_mission_complete_ui))))
    (:then_1
      (UserInterface|Viewport|AddtoPlayerScreen (Variables|Default|GetBP_OC_Game_UI)))
    (:then_2
      (Utilities|Time|SetTimerbyFunctionName 0 "CountTime" 1.0 true))
    (:then_3
      (Input|SetInputModeGameOnly (Game|GetPlayerController 0)))))

(event Collision|EventActorBeginOverlap
  (params (OtherActor :type Actor%20Object%20Reference)))

(event EventTick
  (params (DeltaSeconds :type Float%20%28single-precision%29)))

(fn ConstructionScript)

(fn CountTime
  (bind _returnvalue (Game|GetPlayerController 0))
  (Utilities|FlowControl|Sequence
    (:then_0
      (bind _result (Math|Integer|DecrementInt (Variables|Default|Get현재시간))
        (:%20%20
          (bind _output_get (Variables|Default|Set현재시간 _result))
          (Default|SetTime (Variables|Default|GetBP_OC_Game_UI) _output_get))))
    (:then_1
      (if (<= (Variables|Default|Get현재시간) 0)
        (Utilities|Time|ClearTimerbyFunctionName 0 "CountTime")
        (Variables|/Script/Engine.PlayerController|SetbShowMouseCursor _returnvalue true)
        (UserInterface|Viewport|AddtoPlayerScreen (Variables|Default|GetBP_TimeOver_UI))
        (Input|SetInputModeUIOnly _returnvalue 0 "DoNotLock")))
    (:then_2
      (if (>= (Variables|Default|GetGarbage%20Point) 100)
        (UserInterface|Viewport|AddtoPlayerScreen (Variables|Default|GetBP_MissionComplete_UI))
        (Input|SetInputModeUIOnly (Game|GetPlayerController 0) 0 "DoNotLock")))))

(fn ShowGarbagePoints
  (params (garbagePoints :type Integer))
  (bind _output_get (Variables|Default|SetGarbage%20Point garbagePoints))
  (Default|ShowGabage (Variables|Default|GetBP_OC_Game_UI) _output_get))